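; MovementPlayer moves the player pawn through an ordered array of Target actors.
; Each Tick, while Continue is true, it offsets the pawn by Speed along the normalized direction to the current target, without sweep or delta-time scaling.
; The world-space direction is applied as a local offset.
; Within Treshold distance it advances the index, and a Gate closes after the last target to stop movement.
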(event `self.ReceiveTick`
  (params (DeltaSeconds :type "Float (single-precision)"))
  (`self.Moveto1`))

(event `Moveto1`
  (bind _returnvalue (`GameplayStatics.GetPlayerPawn` 0))
  (bind _returnvalue_2 (- (`self.K2_GetActorLocation` (`|GetArrayItem` (`self.Target`) (`self.i`))) (`self.K2_GetActorLocation` _returnvalue)))
  (`/Engine/EditorBlueprintResources/StandardMacros.Gate` false :!label _label
    (:`Exit`
      (if (`self.continue`)
        (if (>= (`KismetMathLibrary.VSize` _returnvalue_2) (`self.treshold`))
          (`self.K2_AddActorLocalOffset` _returnvalue (* (`KismetMathLibrary.Normal` _returnvalue_2) (`self.speed`)) false false)
          (else
            (bind _result (`/Engine/EditorBlueprintResources/StandardMacros.IncrementInt` (`self.i`))
              (:`  `
                (if (>= _result (`KismetArrayLibrary.Array_Length` (`self.Target`)))
                  (goto _label :!via `Close`))))))))))

(fn `UserConstructionScript`)